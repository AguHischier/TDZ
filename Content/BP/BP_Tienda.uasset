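; BP_Tienda is a shop actor that opens the store interface when the player interacts while nearby.
; A Sphere overlap enables and disables input on the actor, limiting the Interaccion action to that range.
; Interaccion creates Widget_Tienda on first use or makes the existing one visible, then pauses the game and shows the mouse cursor.
; BeginPlay caches the BP_PJ player character and attempts a cast on a stored widget reference.
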(event `self.ReceiveBeginPlay`
  (bind _asbp_pj (cast `/Game/BP/BP_PJ` (`GameplayStatics.GetPlayerCharacter` 0)))
  (set `self.As BP PJ` _asbp_pj)
  (bind _aswidget_tienda (cast `/Game/BP/Widgets/Widget_Tienda` (`self.As Widget Tienda`)))
  (set `self.As Widget Tienda` _aswidget_tienda))

(event `InputAction|Interaccion`
  (params (Key :type "Key Structure"))
  (bind _returnvalue (`GameplayStatics.GetPlayerController` 0))
  (:`Pressed`
    (`/Engine/EditorBlueprintResources/StandardMacros.IsValid` (stale _returnvalue_2)
      (:`Is Valid`
        (`Widget.SetVisibility` (stale _returnvalue_2) "Visible")
        (`GameplayStatics.SetGamePaused` true)
        (set `PlayerController.bShowMouseCursor` true _returnvalue))
      (:`Is Not Valid`
        (bind _returnvalue_2 (`|CreateWidget` "/Game/BP/Widgets/Widget_Tienda.Widget_Tienda_C" _returnvalue))
        (`UserWidget.AddToViewport` _returnvalue_2 0)
        (`GameplayStatics.SetGamePaused` true)
        (set `PlayerController.bShowMouseCursor` true _returnvalue)))))

(event `self.Sphere.OnComponentBeginOverlap`
  (params (OverlappedComponent :type "PrimitiveComponent Object Reference") (OtherActor :type "Actor Object Reference") (OtherComp :type "PrimitiveComponent Object Reference") (OtherBodyIndex :type Integer) (bFromSweep :type Boolean) (SweepResult :type "HitResult Structure (by ref)"))
  (`self.EnableInput` (`GameplayStatics.GetPlayerController` 0)))

(event `self.Sphere.OnComponentEndOverlap`
  (params (OverlappedComponent :type "PrimitiveComponent Object Reference") (OtherActor :type "Actor Object Reference") (OtherComp :type "PrimitiveComponent Object Reference") (OtherBodyIndex :type Integer))
  (`self.DisableInput` (`GameplayStatics.GetPlayerController` 0)))

(fn `UserConstructionScript`)