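; BP_Pistola1 is a pistol item actor that the player can pick up through interaction.
; On BeginPlay it runs the parent logic, then passes an initial state to EstadodelArma (weapon state).
; EnInteraccion calls AgarrarArma (grab weapon) on the interacting player, then passes a second enum state to EstadodelArma.
; EstadodelArma has an empty body here, and the construction script only calls its parent.
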(event `self.ReceiveBeginPlay`
  (`parent.ReceiveBeginPlay`)
  (`self.EstadodelArma` "NewEnumerator0"))

(event `/Game/Elementos_Interacciones/Interacciones.EnInteraccion`
  (params (Player :type "/Game/BP/BP_PJ Object Reference"))
  (`/Game/BP/BP_PJ.AgarrarArma` Player null)
  (`self.EstadodelArma` "NewEnumerator1"))

(fn `EstadodelArma`
  (params (EstadodelArma :type "/Game/BP/Items/Armas/EstadodelArma Enum" :default "NewEnumerator0")))

(fn `UserConstructionScript`
  (`parent.UserConstructionScript`))