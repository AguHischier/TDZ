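; BP_Armas is a pickup weapon that the player can equip, drop, fire and reload.
; A Drop/Equipada state toggles physics and collision, starting dropped; interaction hands the weapon to the player, equips it and can advance the tutorial.
; Firing plays a sound and spawns two actors at the muzzle, one given velocity toward a distant camera-forward point.
; Separate functions decrement the magazine and refill it from reserve ammo.
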(event `self.ReceiveBeginPlay`
  (`parent.ReceiveBeginPlay`)
  (`self.EstadodelArma` "NewEnumerator0"))

(event `/Game/Elementos_Interacciones/Interacciones.EnInteraccion`
  (params (Player :type "/Game/BP/BP_PJ Object Reference"))
  (`|ExecutionSequence`
    (:`then_0`
      (`/Game/BP/BP_PJ.AgarrarArma` Player self)
      (`self.EstadodelArma` "NewEnumerator1"))
    (:`then_1`
      (`/Engine/EditorBlueprintResources/StandardMacros.DoOnce` false :!label _label
        (:`Completed`
          (if (`/Game/BP/BP_PJ.Tuto2` Player)
            (`Widget.SetVisibility` (`/Game/BP/BP_PJ.AyudaWid` Player) "Hidden")
            (set `/Game/BP/BP_PJ.Tuto3` true Player)
            (else
              (goto _label :!via `Reset`))))))))

(fn `DescontarBalaAlDisparar`
  (bind _balasencargador (`self.BalasEnCargador`))
  (if (not (<= _balasencargador 0))
    (`/Engine/EditorBlueprintResources/StandardMacros.DecrementInt` _balasencargador)))

(fn `Disparo`
  (params (PlayerCamera :type "CameraComponent Object Reference"))
  (bind _returnvalue (`SceneComponent.GetSocketLocation` (`self.SkeletalMesh`) "SOCKET_Muzzle"))
  (`|SpawnActorFromClass` "/Game/BP/Items/BP_Bala.BP_Bala_C" (`KismetMathLibrary.MakeTransform` _returnvalue) "Undefined" "OverrideRootScale" null (* (`KismetMathLibrary.Normal` (- (+ (`SceneComponent.K2_GetComponentLocation` PlayerCamera) (* (`SceneComponent.GetForwardVector` PlayerCamera) 10000.0)) _returnvalue)) 10000.0) null)
  (`GameplayStatics.PlaySoundAtLocation` "/Game/Audio/Pistola.Pistola" _returnvalue (struct) 1.0 1.0 0.0 null null null) ; Play firing sound
  (`|SpawnActorFromClass` "/Game/BP/Items/BP_MuzzleFlash.BP_MuzzleFlash_C" (`KismetMathLibrary.MakeTransform` _returnvalue) "Undefined" "OverrideRootScale" null null))

(fn `Drop`
  (`self.EstadodelArma` "NewEnumerator0"))

(fn `EstadodelArma`
  (params (EstadodelArma :type "/Game/BP/Items/Armas/EstadodelArma Enum" :default "NewEnumerator0"))
  (bind _skeletalmesh (`self.SkeletalMesh`))
  (bind _skeletalmesh_2 (`self.SkeletalMesh`))
  (bind _output_get (set `self.Estadodel Arma` EstadodelArma))
  (switch `/Game/BP/Items/Armas/EstadodelArma` _output_get
    (:`NewEnumerator0`
      (`PrimitiveComponent.SetCollisionProfileName` (`self.Sphere`) "OverlapAllDynamic" true)
      (`PrimitiveComponent.SetSimulatePhysics` _skeletalmesh_2 true)
      (`PrimitiveComponent.SetCollisionProfileName` _skeletalmesh_2 "DroppedGun" true))
    (:`NewEnumerator1`
      (`PrimitiveComponent.SetCollisionProfileName` (`self.Sphere`) "NoCollision" true)
      (`PrimitiveComponent.SetSimulatePhysics` _skeletalmesh false)
      (`PrimitiveComponent.SetCollisionProfileName` _skeletalmesh "NoCollision" true)
      (`SceneComponent.ResetRelativeTransform` _skeletalmesh))))

(fn `ObtenerTextoAttach`
  (returns (Componente :type "SceneComponent Object Reference"))
  (return (`self.SkeletalMesh`)))

(fn `ObtenerTextoInteraccion`
  (returns (Texto :type Text))
  (return "Pick Up"))

(fn `Recargar`
  (bind _returnvalue (- (`self.BalasEnInventario`) (- (`self.BalasTotaldelCargador`) (`self.BalasEnCargador`))))
  (if (< _returnvalue 0)
    (set `self.BalasEnCargador` (+ (`self.BalasEnCargador`) (`self.BalasEnInventario`)))
    (set `self.BalasEnInventario` 0)
    (else
      (set `self.BalasEnInventario` _returnvalue)
      (set `self.BalasEnCargador` (`self.BalasTotaldelCargador`)))))

(fn `UserConstructionScript`
  (`parent.UserConstructionScript`))