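; BP_AgarrarBAlas is an ammo pickup that adds bullets to the player's inventory on contact.
; Overlapping its sphere with BP_PJ adds CargarBala to BalasEnInventario, then destroys the pickup.
; It also advances the tutorial: when Tuto3 is set, a DoOnce hides the help widget and sets Tuto4, otherwise the DoOnce resets.
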(event `self.Sphere.OnComponentBeginOverlap`
  (params (OverlappedComponent :type "PrimitiveComponent Object Reference") (OtherActor :type "Actor Object Reference") (OtherComp :type "PrimitiveComponent Object Reference") (OtherBodyIndex :type Integer) (bFromSweep :type Boolean) (SweepResult :type "HitResult Structure (by ref)"))
  (bind _asbp_pj (cast `/Game/BP/BP_PJ` OtherActor))
  (`|ExecutionSequence`
    (:`then_0`
      (`/Engine/EditorBlueprintResources/StandardMacros.DoOnce` false :!label _label
        (:`Completed`
          (if (`/Game/BP/BP_PJ.Tuto3` _asbp_pj)
            (`Widget.SetVisibility` (`/Game/BP/BP_PJ.AyudaWid` _asbp_pj) "Hidden")
            (set `/Game/BP/BP_PJ.Tuto4` true _asbp_pj)
            (else
              (goto _label :!via `Reset`))))))
    (:`then_1`
      (set `/Game/BP/BP_PJ.BalasEnInventario` (+ (`/Game/BP/BP_PJ.BalasEnInventario` _asbp_pj) (`self.CargarBala`)) _asbp_pj)
      (`self.K2_DestroyActor`))))

(fn `UserConstructionScript`)