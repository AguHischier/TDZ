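; BP_Tabernero is a tavern keeper NPC that opens a shop interface when the player enters its ShopTrigger.
; Overlap blends the camera to the actor, switches to UI-only input with a cursor and hides the player character.
; After a short delay it shows or creates the Tabernero widget, pre-creating a hidden Tienda shop widget alongside it.
; A DoOnce prevents retriggering until the player leaves; an unconnected pause-based shop path never runs.
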(event `self.ShopTrigger.OnComponentBeginOverlap`
  (params (OverlappedComponent :type "PrimitiveComponent Object Reference") (OtherActor :type "Actor Object Reference") (OtherComp :type "PrimitiveComponent Object Reference") (OtherBodyIndex :type Integer) (bFromSweep :type Boolean) (SweepResult :type "HitResult Structure (by ref)"))
  (bind _returnvalue (`GameplayStatics.GetPlayerController` 0))
  (if (== OtherActor (`GameplayStatics.GetPlayerCharacter` 0))
    (`/Engine/EditorBlueprintResources/StandardMacros.DoOnce` false :!label _label
      (:`Completed`
        (`PlayerController.SetViewTargetWithBlend` (`GameplayStatics.GetPlayerController` 0) self 1.0 "VTBlend_Linear" 0.0 false)
        (`WidgetBlueprintLibrary.SetInputMode_UIOnlyEx` _returnvalue (`self.Tienda_Wid`))
        (set `PlayerController.bShowMouseCursor` true _returnvalue)
        (`self.SetActorHiddenInGame` (`GameplayStatics.GetPlayerCharacter` 0) true)
        (`KismetSystemLibrary.Delay` 1.2)
        (`/Engine/EditorBlueprintResources/StandardMacros.IsValid` (stale _returnvalue_2)
          (:`Is Valid`
            (`Widget.SetVisibility` (stale _returnvalue_2) "Visible"))
          (:`Is Not Valid`
            (bind _returnvalue_2 (`|CreateWidget` "/Game/BP/Widgets/Widget_Tabernero.Widget_Tabernero_C" (`GameplayStatics.GetPlayerController` 0)))
            (`UserWidget.AddToViewport` _returnvalue_2 0)
            (`/Engine/EditorBlueprintResources/StandardMacros.IsValid` (stale _returnvalue_3)
              (:`Is Not Valid`
                (bind _returnvalue_3 (`|CreateWidget` "/Game/BP/Widgets/Widget_Tienda.Widget_Tienda_C" (`GameplayStatics.GetPlayerController` 0)))
                (`UserWidget.AddToViewport` _returnvalue_3 0)
                (`Widget.SetVisibility` _returnvalue_3 "Hidden")))))))))

(event `self.ShopTrigger.OnComponentEndOverlap`
  (params (OverlappedComponent :type "PrimitiveComponent Object Reference") (OtherActor :type "Actor Object Reference") (OtherComp :type "PrimitiveComponent Object Reference") (OtherBodyIndex :type Integer))
  (if (== OtherActor (`GameplayStatics.GetPlayerCharacter` 0))
    (goto _label :!via `Reset`)))

(event `InputAction|Interaccion`
  (params (Key :type "Key Structure")))

(fn `UserConstructionScript`)