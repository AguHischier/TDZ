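; BP_Partes is a collectible portal part that the BP_PJ player picks up by overlapping its sphere.
; On overlap it increments the player's CantidadPartes count, updates the mission text when a specific count is reached, and destroys itself.
; It also advances the tutorial once the Tuto6 flag is set, hiding the help widget and setting Tuto7, with a DoOnce that resets otherwise.
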(event `self.Sphere1.OnComponentBeginOverlap`
  (params (OverlappedComponent :type "PrimitiveComponent Object Reference") (OtherActor :type "Actor Object Reference") (OtherComp :type "PrimitiveComponent Object Reference") (OtherBodyIndex :type Integer) (bFromSweep :type Boolean) (SweepResult :type "HitResult Structure (by ref)"))
  (bind _asbp_pj (cast `/Game/BP/BP_PJ` OtherActor))
  (`|ExecutionSequence`
    (:`then_0`
      (`/Engine/EditorBlueprintResources/StandardMacros.DoOnce` false :!label _label
        (:`Completed`
          (if (`/Game/BP/BP_PJ.Tuto6` _asbp_pj)
            (`Widget.SetVisibility` (`/Game/BP/BP_PJ.AyudaWid` _asbp_pj) "Hidden")
            (set `/Game/BP/BP_PJ.Tuto7` true _asbp_pj)
            (else
              (goto _label :!via `Reset`))))))
    (:`then_1`
      (bind _result (`/Engine/EditorBlueprintResources/StandardMacros.IncrementInt` (`/Game/BP/BP_PJ.CantidadPartes` _asbp_pj))
        (:`  `
          (if (== _result 1)
            (set `/Game/BP/BP_PJ.MisionActual` "Find parts to repair the portal. \nFind the Portal" _asbp_pj))
          (`self.K2_DestroyActor`))))))

(fn `UserConstructionScript`)